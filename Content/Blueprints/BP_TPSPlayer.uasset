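; BP_TPSPlayer is the third-person shooter player Blueprint, linking player state to the HUD and handling the sniper weapon's visual swap.
; The MakeHPtoPercent event calls its parent, then pushes the HP percent to MainUI on BP_TPSGameMode.
; ChangeWeapon forwards the grenade flag to the same UI.
; The sniper input hides the gun mesh and shows the sniper; the reverse swap exists but is unconnected.
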(event Input|EnhancedActionEvents|EnhancedInputActionIA_TPSSniperGun
  (params (ActionValue :type Boolean) (ElapsedSeconds :type Float%20%28double-precision%29) (TriggeredSeconds :type Float%20%28double-precision%29) (InputAction :type Input%20Action%20Object%20Reference :default "/Game/TPSInput/IA_TPSSniperGun.IA_TPSSniperGun"))
  (:Started
    (Rendering|SetVisibility (Variables|Default|GetgunMeshComp) false false)
    (Rendering|SetVisibility (Variables|Default|GetsniperComp) true false)))

(event EventBeginPlay)

(event EventMakeHPtoPercent
  (|CallParentFunction)
  (bind _asbp_tpsgame_mode (Utilities|Casting|CastToBP_TPSGameMode (Game|GetGameMode)))
  (Default|SetHP (Variables|/Game/Blueprints/BP_TPSGameMode.BP_TPSGameMode_C|GetMainUI _asbp_tpsgame_mode) (Variables|Default|Getpercent)))

(event EventChangeWeapon
  (params (isGrenade :type Boolean))
  (bind _asbp_tpsgame_mode (Utilities|Casting|CastToBP_TPSGameMode (Game|GetGameMode)))
  (Default|ChangeWeapon (Variables|/Game/Blueprints/BP_TPSGameMode.BP_TPSGameMode_C|GetMainUI _asbp_tpsgame_mode) isGrenade))

(fn ConstructionScript)